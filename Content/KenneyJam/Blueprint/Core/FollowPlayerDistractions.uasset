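; Distraction actor that shadows the player and periodically spawns a Bullet at a random point around them.
; A fast looping timer snaps it to the player pawn's location, while a second looping timer, its interval randomized once at BeginPlay, drives attacks.
; Each attack randomizes the Sphere radius, destroys the previous bullet and spawns one on that sphere, rotated by a look-at from actor center to player.
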(event Custom|Attack
  (Components|Sphere|SetSphereRadius (Variables|Default|GetSphere) (Math|Random|RandomFloatinRange 5.0 8e+01) true)
  (Utilities|IsValid (Variables|Default|GetBullet)
    (:Is%20Valid
      (Actor|DestroyActor (Variables|Default|GetBullet))
      (Variables|Default|SetBullet 0))
    (:Is%20Not%20Valid
      _))
  (bind _output_get (Variables|Default|SetSurface%20Normal (Math|Random|RandomUnitVector)))
  (bind _returnvalue (Game|SpawnActorfromClass "/Game/KenneyJam/Blueprint/Core/Bullet.Bullet_C" (Math|Transform|MakeTransform (+ (* _output_get (.SphereRadius (Collision|GetComponentBounds (Variables|Default|GetSphere)))) (Transformation|GetActorLocation)) (Math|Rotator|FindLookatRotation (Transformation|GetActorLocation) (Transformation|GetActorLocation (Game|Player|GetPlayerPawn 0))) "1,1,1") "Undefined" 0 0))
  (Variables|Default|SetBullet _returnvalue))

(event Custom|Follow
  (Transformation|SetActorLocation (Transformation|GetActorLocation (Game|Player|GetPlayerPawn 0)) false false))

(event EventBeginPlay
  (Utilities|Time|SetTimerbyFunctionName 0 "Follow" 0.001 true)
  (Utilities|Time|SetTimerbyFunctionName 0 "Attack" (Math|Random|RandomFloatinRange 1.0 5.0) true))

(fn ConstructionScript)