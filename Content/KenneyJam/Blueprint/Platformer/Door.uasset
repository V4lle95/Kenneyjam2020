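; A clickable door actor in a platformer that teleports the player character to a linked TeleportLocation.
; Clicking the Door component uses SimpleMoveToLocation to send the player controller to the Box component's position.
; When the player character begins overlapping the actor, it teleports to TeleportLocation and faces that target's forward direction.
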(event OnClicked(Door)
  (params (TouchedComponent :type Primitive%20Component%20Object%20Reference) (ButtonPressed :type Key%20Structure :default "None"))
  (AI|Navigation|SimpleMovetoLocation (Game|GetPlayerController 0) (Transformation|GetWorldLocation (Variables|Default|GetBox))))

(event EventBeginPlay)

(event Collision|EventActorBeginOverlap
  (params (OtherActor :type Actor%20Object%20Reference))
  (bind _teleport_location (Variables|Default|GetTeleport%20Location))
  (if (== OtherActor (Game|GetPlayerCharacter 0))
    (Transformation|Teleport OtherActor (Transformation|GetActorLocation _teleport_location) (Math|Conversions|RotationFromXVector (Transformation|GetActorForwardVector _teleport_location)))))

(event EventTick
  (params (DeltaSeconds :type Float%20%28single-precision%29)))

(fn ConstructionScript)