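; Platformer cannon that automatically fires a bullet on a fixed interval.
; A looping timer set to TimeToFire calls FakeTick, which spawns a Bullet at the Arrow component, facing along its forward vector.
; Each shot also restarts the Animation timeline, which lerps the Scene component's scale between uniform and narrowed on Y and Z.
; The construction script uses TimeToFire directly as that timeline's play rate.
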(event Custom|Fake%20Tick
  (bind _arrow (Variables|Default|GetArrow))
  (Utilities|FlowControl|Sequence
    (:then_0
      (bind _returnvalue (Game|SpawnActorfromClass "/Game/KenneyJam/Blueprint/Core/Bullet.Bullet_C" (Math|Transform|MakeTransform (Transformation|GetWorldLocation _arrow) (Math|Conversions|RotationFromXVector (Math|Vector|GetForwardVector _arrow)) "1,1,1") "AdjustIfPossibleButDontSpawnIfColliding" 0 0))
      (Variables|Default|SetBullet _returnvalue))
    (:then_1
      (bind _alpha (Timeline|Animation PlayFromStart)
        (:Update
          (Transformation|SetRelativeScale3D (Variables|Default|GetScene) (Math|Vector|Lerp(Vector) "2.000000,2.000000,2.000000" "2.000000,0.200000,0.200000" _alpha)))))))

(event EventBeginPlay
  (Utilities|Time|SetTimerbyFunctionName 0 "Fake Tick" (Variables|Default|GetTime%20to%20Fire) true))

(fn ConstructionScript
  (Components|Timeline|SetPlayRate (Variables|Default|GetAnimation) (Variables|Default|GetTime%20to%20Fire)))