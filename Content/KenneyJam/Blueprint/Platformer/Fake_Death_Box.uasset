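; Fake death volume for a platformer level that punishes the player without killing them.
; When the player pawn overlaps it, the pawn is teleported to the ActorTeleports location and facing, a loser sound plays, and a FollowPlayerDistractions actor spawns.
; The construction script resizes the Trigger box from the BoxSize variable.
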(event Collision|EventActorBeginOverlap
  (params (OtherActor :type Actor%20Object%20Reference))
  (bind _actor_teleports (Variables|Default|GetActor%20Teleports))
  (if (== OtherActor (Game|Player|GetPlayerPawn 0))
    (Transformation|Teleport OtherActor (Transformation|GetActorLocation _actor_teleports) (Math|Conversions|RotationFromXVector (Transformation|GetActorForwardVector _actor_teleports)))
    (Audio|PlaySound2D "/Game/KenneyJam/Audio/loser.loser" 1.0 1.0 0.0 0 0)
    (Game|SpawnActorfromClass "/Game/KenneyJam/Blueprint/Core/FollowPlayerDistractions.FollowPlayerDistractions_C" (Math|Transform|MakeTransform "0, 0, 0" "0, 0, 0" "1,1,1") "Undefined" 0 0)))

(fn ConstructionScript
  (Components|Box|SetBoxExtent (Variables|Default|GetTrigger) (Variables|Default|GetBox%20Size) true))