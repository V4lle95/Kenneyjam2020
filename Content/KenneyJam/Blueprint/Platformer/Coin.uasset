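; Coin pickup actor for a platformer that gives the player a coin and may trigger a jump scare.
; When the player pawn overlaps it, it adds one coin through the player, plays a glitch sound, has a 50% chance to show a JumpScare widget, then expires after a short lifespan.
; Clicking the coin sends the player controller's pawn walking to it via SimpleMoveToActor.
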(event OnClicked(Coin)
  (params (TouchedComponent :type Primitive%20Component%20Object%20Reference) (ButtonPressed :type Key%20Structure :default "None"))
  (AI|Navigation|SimpleMovetoActor (Game|GetPlayerController 0) self))

(event Collision|EventActorBeginOverlap
  (params (OtherActor :type Actor%20Object%20Reference))
  (if (== OtherActor (Game|Player|GetPlayerPawn 0))
    (Utilities|FlowControl|Sequence
      (:then_0
        (bind _player (CallFunction|GetPlayer))
        (Default|Add/RemoveCoins _player 1)
        (Audio|PlaySound2D "/Game/KenneyJam/Audio/glitch_001.glitch_001" 1.0 1.0 0.0 0 0))
      (:then_1
        (if (>= (Math|Random|RandomFloatinRange 0.0 2.0) 1.0)
          (bind _returnvalue (UserInterface|CreateWidget "/Game/KenneyJam/Widget/JumpScare.JumpScare_C"))
          (UserInterface|Viewport|AddtoViewport _returnvalue 1)))
      (:then_2
        (Actor|SetLifeSpan 0.5)))))

(fn ConstructionScript)